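; House_V8 is a clickable house actor that identifies which material slot of a mesh lies under the camera's view.
; OnClicked runs a persistent-debug complex trace from the camera, then prints indices of materials whose names match the hit face's material.
; The trace end is the scaled forward vector, without the camera location added.
; MultiGate material cycling and dynamic material creation are unconnected; a mouse-down function prints cursor position.
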(event OnClicked(House_V8)
  (params (TouchedComponent :type Primitive%20Component%20Object%20Reference) (ButtonPressed :type Key%20Structure))
  (bind _returnvalue (Game|GetPlayerCameraManager 0))
  (bind (_outhit _returnvalue_2) (Collision|LineTraceByChannel (Transformation|GetWorldLocation (Variables|/Script/Engine.Actor|GetRootComponent _returnvalue)) (* (Math|Vector|GetForwardVector (Transformation|GetWorldRotation (Variables|/Script/Engine.Actor|GetRootComponent _returnvalue))) 100000) "TraceTypeQuery1" true 0 "Persistent"))
  (bind _asstatic_mesh_component (Utilities|Casting|CastToStaticMeshComponent (.HitComponent (Collision|BreakHitResult _outhit)))
    (:then
      (for (_array_element _array_index) (Rendering|Material|GetMaterials _asstatic_mesh_component)
        (if (Utilities|Enum|Equal(Enum) (Utilities|GetObjectName _array_element) (Utilities|GetObjectName (.ReturnValue (Class|PrimitiveComponent|GetMaterialfromCollisionFaceIndex (.HitComponent (Collision|BreakHitResult _outhit)) (.FaceIndex (Collision|BreakHitResult _outhit))))))
          (Development|PrintString (Utilities|String|ToString(Integer) _array_index)))))
    (:CastFailed
      (Development|PrintString "Failed"))))

(event EventBeginPlay)

(event Collision|EventActorBeginOverlap
  (params (OtherActor :type Actor%20Object%20Reference)))

(fn ConstructionScript)

(fn OnMouseButtonDown
  (params (My%20Geometry :type Geometry%20Structure) (Mouse%20Event :type Input%20Event%20Structure) (Player%20Controller :type Player%20Controller%20Object%20Reference))
  (Development|PrintString (Utilities|String|ToString(Boolean) (.ReturnValue (Game|Player|GetMousePosition Player%20Controller))))
  (return (Class|WidgetBlueprintLibrary|Handled)))