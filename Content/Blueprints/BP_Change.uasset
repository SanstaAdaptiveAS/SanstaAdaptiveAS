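; BP_Change is an actor that changes the material on its UnrealTest07 mesh when that mesh is clicked.
; A looping, ordered MultiGate cycles material slot 0 through paint, plaster and ceramic tile finishes.
; A second MultiGate for parquet finishes on slot 2 sits behind a Branch with a constant true condition, so it never runs.
; Unconnected nodes for material index and collision face lookup are left unused.
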(event OnClicked(UnrealTest_07)
  (params (TouchedComponent :type Primitive%20Component%20Object%20Reference) (ButtonPressed :type Key%20Structure))
  (bind _unrealtest_07 (Variables|Default|GetUnrealTest_07))
  (if true
    (Utilities|FlowControl|MultiGate false true -1
      (:Out%200
        (Rendering|Material|SetMaterial _unrealtest_07 0 "/Game/Materials/Wall_paint/Wall_paint.Wall_paint"))
      (:Out%201
        (Rendering|Material|SetMaterial _unrealtest_07 0 "/Game/Materials/Spanish_Plaster/Spanish_Plaster__MAT.Spanish_Plaster__MAT"))
      (:Out%202
        (Rendering|Material|SetMaterial _unrealtest_07 0 "/Game/Materials/Floral_Ceramic_Tiles/Floral_Ceramic_Tiles_MAT.Floral_Ceramic_Tiles_MAT")))
    (else
      (Utilities|FlowControl|MultiGate false true -1
        (:Out%200
          (Rendering|Material|SetMaterial _unrealtest_07 2 "/Game/Materials/Wood_Parquet_Mahogany/Parquet_Mahogany_MAT.Parquet_Mahogany_MAT"))
        (:Out%201
          (Rendering|Material|SetMaterial _unrealtest_07 2 "/Game/Materials/Wood_parquet/Wood_parquet.Wood_parquet"))))))

(event Collision|EventActorBeginOverlap
  (params (OtherActor :type Actor%20Object%20Reference)))

(fn ConstructionScript)